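; Player controller for classic PvE chess that lets the player pick a move with the mouse during their turn.
; StartTurn spawns a selector actor that Tick snaps to the BP_Grid tile under the cursor; two left clicks set the from and to tiles.
; CheckMove only detects pawn promotion, opening the HUD's promotion widget to choose a piece.
; MakeMove stores the move and tells the game mode to cycle turns.
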(event `self.ReceiveBeginPlay`)

(event `SetPlayerID`
  (params (PlayerID :type Integer))
  (set `self.Player ID` PlayerID))

(event `StartTurn`
  (set `self.Figure Type` 0)
  (if (`KismetSystemLibrary.IsValid` (`self.PlayerHUD`))
    (`self.SetMyTurn` true :!label _label)
    (set `self.isFirstTileSelection` true)
    (`self.SelectTile`)
    (elif (`self.IsLocalPlayerController`)
      (bind _asbp_hud (`/Game/ModeBP/BML_PlayerController.GetBP_HUD` 10.0)
        (:`Success`
          (set `self.PlayerHUD` _asbp_hud)
          (goto _label))
        (:`Failed`
          (`KismetSystemLibrary.PrintText` "Failed to get hud")))
      (else
        (`KismetSystemLibrary.PrintText` "ERROR" true true (struct :`R` 1.0 :`A` 1.0))))))

(event `EndTurn`
  (`self.SetMyTurn` false))

(event `MakeMove`
  (params (From :type "IntPoint Structure") (To :type "IntPoint Structure") (PromotionType :type Byte))
  (set `self.fromTile` From)
  (set `self.toTile` To)
  (set `self.Figure Type` PromotionType)
  (if (not (`KismetSystemLibrary.IsValid` (`self.GameMode`)))
    (bind _asbp_classic_pv_egame_mode (cast `/Game/ModeBP/Classic/BP_ClassicPvEGameMode` (`GameplayStatics.GetGameMode`)))
    (set `self.GameMode` _asbp_classic_pv_egame_mode))
  (`/Game/ModeBP/Classic/BP_ClassicPvEGameMode.CycleTurns` (`self.GameMode`)))

(event `self.ReceiveTick`
  (params (DeltaSeconds :type "Float (single-precision)"))
  (if (and (`self.isMyTurn`) (not (`self.madeSelection`)))
    (bind _returnvalue (`GameplayStatics.GetActorOfClass` "/Game/ModeBP/BP_Grid.BP_Grid_C"))
    (`/Engine/EditorBlueprintResources/StandardMacros.IsValid` _returnvalue
      (:`Is Valid`
        (bind _id (`/Game/ModeBP/BP_Grid.GetTileIDUnderCursor` _returnvalue 0))
        (bind _selector (`self.Selector`)
          (:`then`
            (bind _value (`BlueprintMapLibrary.Map_Find` (`/Game/ModeBP/BP_Grid.TileTransforms` _returnvalue) _id))
            (bind (_sweephitresult _returnvalue_2) (`self.K2_SetActorTransform` _selector (`KismetMathLibrary.MakeTransform` (+ (.location _value) (100.0 100.0 10.0)) (.rotation _value) (.scale _value)) false false)))
          (:`else`
            (`KismetSystemLibrary.PrintText` "[ERROR] Invalid selector" true true (struct :`R` 1.0 :`A` 1.0))))))))

(event `Key|LeftMouseButton`
  (params (Key :type "Key Structure"))
  (:`Pressed`
    (if (stale `self.ReceiveTick` _returnvalue_2)
      (set `self.madeSelection` true)
      (bind _output_get (set `self.SelectedTile` (stale `self.ReceiveTick` _id)))
      (if (`self.isFirstTileSelection`)
        (set `self.fromTile` _output_get)
        (else
          (set `self.toTile` _output_get)))
      (`self.EndSelection`))))

(event `EndSelection`
  (bind _selector (`self.Selector`))
  (if (`KismetSystemLibrary.IsValid` _selector)
    (`self.K2_DestroyActor` _selector)
    (if (`self.isFirstTileSelection`)
      (set `self.isFirstTileSelection` false)
      (`self.SelectTile`)
      (else
        (`self.CheckMove` (`self.Player ID`) (`self.fromTile`) (`self.toTile`))))))

(event `ShowPromotionWidget`
  (`/Game/ModeBP/Classic/BP_ClassicHUD.TogglePromotionWidget` (`self.PlayerHUD`)))

(event `SetPromotionFigure`
  (params (FigureType :type Byte))
  (`self.MakeMove` (`self.CheckMoveFromTile`) (`self.CheckMoveToTile`) FigureType)
  (`self.ShowPromotionWidget`))

(event `CheckMove`
  (params (PlayerID :type Integer) (FromTile :type "IntPoint Structure") (ToTile :type "IntPoint Structure"))
  (bind _checkmovetotile_x (break `IntPoint` (`self.CheckMoveToTile`)))
  (set `self.CheckMoveFromTile` FromTile)
  (set `self.CheckMoveToTile` ToTile)
  (bind _returnvalue (`GameplayStatics.GetActorOfClass` "/Game/ModeBP/BP_Grid.BP_Grid_C"))
  (bind _piece (`/Game/ModeBP/BP_Grid.GetPieceAtTile` _returnvalue (`self.CheckMoveFromTile`)))
  (if (and (`KismetMathLibrary.ClassIsChildOf` (`GameplayStatics.GetObjectClass` _piece) "/Game/Pieces/BP_PawnFigure.BP_PawnFigure_C") (== (select `int` (`self.Player ID`) :`0` 7 :`1` 0 :!type "Byte") _checkmovetotile_x))
    (`self.ShowPromotionWidget`)
    (else
      (`self.MakeMove` (`self.CheckMoveFromTile`) (`self.CheckMoveToTile`)))))

(fn `SelectTile`
  (set `self.madeSelection` false)
  (bind _returnvalue (`|SpawnActorFromClass` "/Game/ModeBP/BP_TileSelectionActor.BP_TileSelectionActor_C" (`KismetMathLibrary.MakeTransform` (0.0 0.0 -1000.0)) "AlwaysSpawn" "MultiplyWithRoot" null null))
  (set `self.Selector` _returnvalue))

(fn `SetMyTurn`
  (params (MyTurn :type Boolean))
  (bind _output_get (set `self.isMyTurn` MyTurn))
  (`self.OnTurnChange` _output_get))

(fn `UserConstructionScript`)