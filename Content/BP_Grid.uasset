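; Grid actor that builds a tiled grid and resolves which tile lies under a player's mouse cursor.
; The construction script calls SpawnGrid, adding centered hierarchical instanced mesh tiles and mapping integer coordinates to their transforms.
; Cursor lookup uses a camera-channel trace, falling back to an offset intersection with the grid's horizontal plane.
; That location converts to a tile ID using a fixed 200-unit snap divided by tile size.
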(fn `GetCursorLocation`
  (params (PlayerIndex :type Integer))
  (returns (Location :type "Vector Structure"))
  (bind _returnvalue (`GameplayStatics.GetPlayerController` PlayerIndex))
  (bind (_hitresult _returnvalue_2) (`PlayerController.GetHitResultUnderCursorByChannel` _returnvalue "TraceTypeQuery2" true))
  (bind (_worldlocation _worlddirection) (`PlayerController.DeprojectMousePositionToWorld` _returnvalue))
  (bind (_t _intersection _returnvalue_3) (`KismetMathLibrary.LinePlaneIntersection` _worldlocation (+ _worldlocation (* _worlddirection (9999999.0 9999999.0 9999999.0))) (`KismetMathLibrary.MakePlaneFromPointAndNormal` (`self.Spawn Location Center`) (0.0 0.0 1.0))))
  (if _returnvalue_2
    (return (`.Location` (`GameplayStatics.BreakHitResult` _hitresult)))
    (elif _returnvalue_3
      (return (+ _intersection (-100.0 -100.0 0.0)))
      (else
        (return (-999.0 -999.0 -999.0))))))

(fn `GetTileIDFromWorld`
  (params (Location :type "Vector Structure"))
  (returns (ID :type "IntPoint Structure"))
  (locals (LocationOnGrid :type "Vector Structure") (SnappedLocationOnGrid :type "Vector Structure" :default (0.0 0.0 0.0)))
  (set `local.LocationOnGrid` (- Location (`self.GridBottomLeftCorner`)))
  (set `local.SnappedLocationOnGrid` (`KismetMathLibrary.Vector_SnappedToGrid` (`local.LocationOnGrid`) 200.0))
  (return (`KismetMathLibrary.Conv_Vector2DToIntPoint` (`KismetMathLibrary.Conv_VectorToVector2D` (/ (`local.SnappedLocationOnGrid`) (`self.Tile Size`))))))

(fn `GetTileIDUnderCursor`
  (params (PlayerIndex :type Integer))
  (returns (ID :type "IntPoint Structure"))
  (locals (SelectedTileTransform :type "Transform Structure"))
  (bind _location (`self.GetCursorLocation` PlayerIndex))
  (bind _id (`self.GetTileIDFromWorld` _location))
  (return _id))

(fn `SpawnGrid`
  (params (SpawnLocationCenter :type "Vector Structure") (TileSize :type "Vector Structure") (GridSize :type "Vector2D Structure"))
  (locals (X :type Integer) (Y :type Integer) (TileTransform :type "Transform Structure"))
  (bind (_grid_size_x _grid_size_y) (`KismetMathLibrary.BreakVector2D` (`self.Grid Size`)))
  (bind _grid_size_x_2 (`KismetMathLibrary.BreakVector2D` (`self.Grid Size`)))
  (set `self.Spawn Location Center` SpawnLocationCenter)
  (set `self.Tile Size` TileSize)
  (set `self.Grid Size` GridSize)
  (`StaticMeshComponent.SetStaticMesh` (`self.HierarchicalInstancedStaticMesh`) null)
  (set `self.GridBottomLeftCorner` (- (`self.Spawn Location Center`) (* (/ (`self.Grid Size`) (2.0 2.0)) (`self.Tile Size`))))
  (for _index (range (`KismetMathLibrary.Round` _grid_size_x_2))
    (set `local.X` _index)
    (for _index_2 (range (`KismetMathLibrary.Round` _grid_size_y))
      (set `local.Y` _index_2)
      (bind _output_get (set `local.TileTransform` (`KismetMathLibrary.MakeTransform` (+ (`self.GridBottomLeftCorner`) (* (`self.Tile Size`) (`KismetMathLibrary.MakeVector` (`local.X`) (`local.Y`)))) (struct) (/ (`self.Tile Size`) (200.0 200.0 7.0)))))
      (`BlueprintMapLibrary.Map_Add` (`self.TileTransforms`) (make `IntPoint` (`local.X`) (`local.Y`)) _output_get)
      (`InstancedStaticMeshComponent.AddInstance` (`self.HierarchicalInstancedStaticMesh`) (`local.TileTransform`) false))))

(fn `UserConstructionScript`
  (`self.SpawnGrid` (`self.Spawn Location Center`) (`self.Tile Size`) (`self.Grid Size`)))