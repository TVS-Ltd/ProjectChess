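; BP_ClassicPlayerController is a turn-based player controller that lets its player pick one grid tile per turn.
; StartTurn flags the turn, fires the turn-change call and spawns a selector actor, which Tick snaps to the BP_Grid tile under the cursor with an offset.
; Left click, gated on the last transform result, stores that tile, destroys the selector and asks BP_ClassicGameMode to cycle turns.
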(event `self.ReceiveBeginPlay`)

(event `SetPlayerID`
  (params (PlayerID :type Integer))
  (set `self.Player ID` PlayerID))

(event `StartTurn`
  (`self.SetMyTurn` true)
  (`KismetSystemLibrary.PrintString` (`KismetStringLibrary.Concat_StrStr` "Current turn's Player ID" (`KismetStringLibrary.Conv_IntToString` (`self.Player ID`))) true true (struct :`R` 1.0 :`G` 0.958134 :`A` 1.0))
  (`self.SelectTile`))

(event `EndTurn`
  (`self.SetMyTurn` false))

(event `MakeMove`
  (bind _asbp_classic_game_mode (cast `/Game/BP_ClassicGameMode` (`GameplayStatics.GetGameMode`)))
  (`/Game/BP_ClassicGameMode.CycleTurns` _asbp_classic_game_mode))

(event `self.ReceiveTick`
  (params (DeltaSeconds :type "Float (single-precision)"))
  (if (and (`self.isMyTurn`) (not (`self.madeSelection`)))
    (bind _returnvalue (`GameplayStatics.GetActorOfClass` "/Game/BP_Grid.BP_Grid_C"))
    (bind _id (`/Game/BP_Grid.GetTileIDUnderCursor` _returnvalue 0))
    (bind _selector (`self.Selector`)
      (:`then`
        (bind _value (`BlueprintMapLibrary.Map_Find` (`/Game/BP_Grid.TileTransforms` _returnvalue) _id))
        (bind (_sweephitresult _returnvalue_2) (`self.K2_SetActorTransform` _selector (`KismetMathLibrary.MakeTransform` (+ (.location _value) (100.0 100.0 10.0)) (.rotation _value) (.scale _value)) false true)))
      (:`else`
        (`KismetSystemLibrary.PrintText` "[ERROR] Invalid selector" true true (struct :`R` 1.0 :`A` 1.0))))))

(event `Key|LeftMouseButton`
  (params (Key :type "Key Structure"))
  (:`Pressed`
    (if (stale `self.ReceiveTick` _returnvalue_2)
      (set `self.madeSelection` true)
      (bind _output_get (set `self.SelectedTile` (stale `self.ReceiveTick` _id)))
      (`KismetSystemLibrary.PrintString` (`KismetStringLibrary.Concat_StrStr` "Player " (`KismetStringLibrary.Conv_IntToString` (`self.Player ID`)) " selected tile: " (`KismetStringLibrary.Conv_IntPointToString` _output_get)) true true (struct :`R` 0.947131 :`G` 1.0 :`A` 1.0))
      (`self.EndSelection`))))

(event `EndSelection`
  (bind _selector (`self.Selector`))
  (if (`KismetSystemLibrary.IsValid` _selector)
    (`self.K2_DestroyActor` _selector)
    (`self.MakeMove`)))

(fn `SelectTile`
  (set `self.madeSelection` false)
  (bind _returnvalue (`|SpawnActorFromClass` "/Game/BP_TileSelectionActor.BP_TileSelectionActor_C" (`KismetMathLibrary.MakeTransform` (0.0 0.0 -1000.0)) "AlwaysSpawn" "MultiplyWithRoot" null null))
  (set `self.Selector` _returnvalue))

(fn `SetMyTurn`
  (params (MyTurn :type Boolean))
  (bind _output_get (set `self.isMyTurn` MyTurn))
  (`self.OnTurnChange` _output_get))

(fn `UserConstructionScript`)