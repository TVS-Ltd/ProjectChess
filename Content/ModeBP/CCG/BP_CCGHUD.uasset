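; CCG mode HUD that creates the main game HUD, promotion and card widgets at BeginPlay and adds them to the viewport.
; The promotion and card widgets share a list, and the card toggle runs on each pass of the loop that adds them.
; ToggleWidget makes them mutually exclusive, collapsing the others and either collapsing the target or showing it with Game and UI input focus.
; The main HUD stays outside this toggling.
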(event `self.ReceiveBeginPlay`
  ;[1 1 1] Game
  (bind _returnvalue (`|CreateWidget` "/Game/Widgets/WB_CCG_HUD.WB_CCG_HUD_C" (`self.GetOwningPlayerController`)))
  (`UserWidget.AddToViewport` _returnvalue 0)
  ;[1 1 1] GameMenus
  (bind _returnvalue_2 (`|CreateWidget` "/Game/Widgets/WB_PromotionWidget.WB_PromotionWidget_C" (`self.GetOwningPlayerController`)))
  (bind _output_get (set `self.WB_PromotionWidget` _returnvalue_2))
  (`KismetArrayLibrary.Array_Add` (`self.WidgetList`) _output_get)
  ;[1 1 1] Card HUD
  (bind _returnvalue_3 (`|CreateWidget` "/Game/Widgets/CardSystem/WB_CardHUD.WB_CardHUD_C" (`self.GetOwningPlayerController`)))
  (bind _output_get_2 (set `self.WB_CardHUDWidget` _returnvalue_3))
  (`KismetArrayLibrary.Array_Add` (`self.WidgetList`) _output_get_2)
  (for _array_element (`self.WidgetList`)
    (`UserWidget.AddToViewport` _array_element 0)
    (`self.ToogleCardHUDWidget`)))

(event `TogglePromotionWidget`
  (`self.ToggleWidget` (`self.WB_PromotionWidget`)))

(event `ToogleCardHUDWidget`
  (`self.ToggleWidget` (`self.WB_CardHUDWidget`)))

(fn `FocusWidget`
  (`Widget.SetVisibility` (`self.ActiveWidget`) "SelfHitTestInvisible")
  (`WidgetBlueprintLibrary.SetInputMode_GameAndUIEx` (`self.GetOwningPlayerController`) (`self.ActiveWidget`)))

(fn `ToggleWidget`
  (params (TargetWidget :type "UserWidget Object Reference"))
  (`/Engine/EditorBlueprintResources/StandardMacros.IsValid` TargetWidget
    (:`Is Valid`
      (set `self.ActiveWidget` (`local.TargetWidget`))
      (for _array_element (`self.WidgetList`)
        (`/Engine/EditorBlueprintResources/StandardMacros.IsValid` _array_element
          (:`Is Valid`
            (if (== (`self.ActiveWidget`) _array_element)
              (if (`Widget.IsVisible` (`self.ActiveWidget`))
                (`Widget.SetVisibility` (`self.ActiveWidget`) "Collapsed")
                (else
                  (`self.FocusWidget`)))
              (elif (`Widget.IsVisible` _array_element)
                (`Widget.SetVisibility` _array_element "Collapsed")))))))))

(fn `UserConstructionScript`)