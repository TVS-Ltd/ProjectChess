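; Chess-style board actor that builds the tile grid, tracks pieces and executes moves and captures.
; The construction script lays out tiles as hierarchical instanced meshes and maps each coordinate to its transform.
; On BeginPlay, the authority spawns pawns and rooks for two players into a flat 64-slot board array.
; Cursor traces resolve to tile IDs, while PerformMove teleports pieces, destroys occupants and updates the array without checking move legality.
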(event `self.ReceiveBeginPlay`
  (if (`self.HasAuthority`)
    (`KismetArrayLibrary.Array_Resize` (`self.BoardState`) 64)
    (for _index (range 2)
      (`self.SpawnPawns` _index)
      (`self.SpawnRooks` _index))))

(fn `AddPieceToBoardState`
  (params (Piece :type "/Game/ClassicModeBP/BP_FigureCharacter Object Reference") (Tile :type "IntPoint Structure"))
  (`KismetArrayLibrary.Array_Set` (`self.BoardState`) (`self.TileToID` Tile) Piece))

(fn `GetCursorLocation`
  (params (PlayerIndex :type Integer))
  (returns (Location :type "Vector Structure"))
  (bind (_worldlocation _worlddirection) (`PlayerController.DeprojectMousePositionToWorld` (`GameplayStatics.GetPlayerController` PlayerIndex)))
  (bind (_outhit _returnvalue) (`KismetSystemLibrary.LineTraceSingle` _worldlocation (+ _worldlocation (* _worlddirection (10000.0 10000.0 10000.0))) "TraceTypeQuery1"))
  (if _returnvalue
    (return (+ (`.Location` (`GameplayStatics.BreakHitResult` _outhit)) (-70.0 -70.0 0.0)))
    (else
      (return (-999.0 -999.0 -999.0)))))

(fn `GetPieceAtTile`
  (params (Tile :type "IntPoint Structure"))
  (returns (Piece :type "/Game/ClassicModeBP/BP_FigureCharacter Object Reference"))
  (bind _id (`self.TileToID` Tile))
  (`KismetSystemLibrary.PrintString` (`KismetStringLibrary.Concat_StrStr` "GettingPiece at ID: " (`KismetStringLibrary.Conv_IntToString` _id)) true true (struct :`R` 1.0 :`G` 0.407399 :`A` 1.0))
  (return (`|GetArrayItem` (`self.BoardState`) _id)))

(fn `GetTileIDFromWorld`
  (params (Location :type "Vector Structure"))
  (returns (ID :type "IntPoint Structure"))
  (locals (LocationOnGrid :type "Vector Structure") (SnappedLocationOnGrid :type "Vector Structure" :default (0.0 0.0 0.0)))
  (set `local.LocationOnGrid` (- Location (`self.GridBottomLeftCorner`)))
  (set `local.SnappedLocationOnGrid` (`KismetMathLibrary.Vector_SnappedToGrid` (`local.LocationOnGrid`) 200.0))
  (return (`KismetMathLibrary.Conv_Vector2DToIntPoint` (`KismetMathLibrary.Conv_VectorToVector2D` (/ (`local.SnappedLocationOnGrid`) (`self.Tile Size`))))))

(fn `GetTileIDUnderCursor`
  (params (PlayerIndex :type Integer))
  (returns (ID :type "IntPoint Structure"))
  (locals (SelectedTileTransform :type "Transform Structure"))
  (bind _location (`self.GetCursorLocation` PlayerIndex))
  (bind _id (`self.GetTileIDFromWorld` _location))
  (return _id))

(fn `MovePieceBoardState`
  (params (FromTile :type "IntPoint Structure") (ToTile :type "IntPoint Structure"))
  (locals (PieceToMove :type "/Game/ClassicModeBP/BP_FigureCharacter Object Reference"))
  (bind _piece (`self.GetPieceAtTile` FromTile))
  (set `local.PieceToMove` _piece)
  (`KismetArrayLibrary.Array_Set` (`self.BoardState`) (`self.TileToID` (`local.FromTile`)))
  (`KismetArrayLibrary.Array_Set` (`self.BoardState`) (`self.TileToID` (`local.ToTile`)) (`local.PieceToMove`)))

(fn `PerformMove`
  (params (FromTile :type "IntPoint Structure") (ToTile :type "IntPoint Structure"))
  (locals (SelectedPiece :type "/Game/ClassicModeBP/BP_FigureCharacter Object Reference") (DestinationPiece :type "/Game/ClassicModeBP/BP_FigureCharacter Object Reference"))
  (bind _piece (`self.GetPieceAtTile` FromTile))
  (set `local.SelectedPiece` _piece)
  (bind _piece_2 (`self.GetPieceAtTile` ToTile))
  (set `local.DestinationPiece` _piece_2)
  (bind _selectedpiece (`local.SelectedPiece`)
    (:`then`
      (`self.K2_SetActorLocation` _selectedpiece (+ (.location (`BlueprintMapLibrary.Map_Find` (`self.TileTransforms`) (`local.ToTile`))) (100.0 100.0 50.0)) false true)
      (bind _destinationpiece (`local.DestinationPiece`)
        (:`then`
          (`self.K2_DestroyActor` _destinationpiece))
        (:`else`
          _))
      (`self.MovePieceBoardState` (`local.FromTile`) (`local.ToTile`)))
    (:`else`
      (`KismetSystemLibrary.PrintText` "[ERROR] Invalid Selected Piece" true true (struct :`R` 1.0 :`A` 1.0)))))

(fn `SpawnGrid`
  (params (SpawnLocationCenter :type "Vector Structure") (TileSize :type "Vector Structure") (GridSize :type "Vector2D Structure"))
  (locals (X :type Integer) (Y :type Integer) (TileTransform :type "Transform Structure"))
  (bind (_grid_size_x _grid_size_y) (`KismetMathLibrary.BreakVector2D` (`self.Grid Size`)))
  (bind _grid_size_x_2 (`KismetMathLibrary.BreakVector2D` (`self.Grid Size`)))
  (set `self.Spawn Location Center` SpawnLocationCenter)
  (set `self.Tile Size` TileSize)
  (set `self.Grid Size` GridSize)
  (`StaticMeshComponent.SetStaticMesh` (`self.HierarchicalInstancedStaticMesh`) null)
  (set `self.GridBottomLeftCorner` (- (`self.Spawn Location Center`) (* (/ (`self.Grid Size`) (2.0 2.0)) (`self.Tile Size`))))
  (for _index (range (`KismetMathLibrary.Round` _grid_size_x_2))
    (set `local.X` _index)
    (for _index_2 (range (`KismetMathLibrary.Round` _grid_size_y))
      (set `local.Y` _index_2)
      (bind _output_get (set `local.TileTransform` (`KismetMathLibrary.MakeTransform` (+ (`self.GridBottomLeftCorner`) (* (`self.Tile Size`) (`KismetMathLibrary.MakeVector` (`local.X`) (`local.Y`)))) (struct) (/ (`self.Tile Size`) (200.0 200.0 7.0)))))
      (`BlueprintMapLibrary.Map_Add` (`self.TileTransforms`) (make `IntPoint` (`local.X`) (`local.Y`)) _output_get)
      (`InstancedStaticMeshComponent.AddInstance` (`self.HierarchicalInstancedStaticMesh`) (`local.TileTransform`) false))))

(fn `SpawnPawns`
  (params (PlayerID :type Integer))
  (locals (Row :type Integer) (Col :type Integer))
  (bind _output_get (set `local.Row` (select `int` PlayerID :`0` 1 :`1` 6)))
  (for _index (range 8)
    (bind _output_get_2 (set `local.Col` _index))
    (bind _returnvalue (`|SpawnActorFromClass` "/Game/Pieces/BP_PawnFigure.BP_PawnFigure_C" (`KismetMathLibrary.MakeTransform` (+ (.location (`BlueprintMapLibrary.Map_Find` (`self.TileTransforms`) (make `IntPoint` _output_get _output_get_2))) (100.0 100.0 50.0))) "AlwaysSpawn" "MultiplyWithRoot" null (`local.PlayerID`) null))
    (`self.AddPieceToBoardState` _returnvalue (make `IntPoint` (`local.Row`) (`local.Col`)))))

(fn `SpawnRooks`
  (params (PlayeriD :type Integer))
  (locals (Row :type Integer) (Col :type Integer))
  (set `local.Row` (select `int` (`local.PlayeriD`) :`0` 0 :`1` 7))
  (`|ExecutionSequence`
    (:`then_0`
      ;[1 1 1] Left
      (bind _output_get (set `local.Col` (select `int` (`local.PlayeriD`) :`0` 0 :`1` 7)))
      (bind _returnvalue (`|SpawnActorFromClass` "/Game/Pieces/BP_RookFigure.BP_RookFigure_C" (`KismetMathLibrary.MakeTransform` (+ (.location (`BlueprintMapLibrary.Map_Find` (`self.TileTransforms`) (make `IntPoint` (`local.Row`) _output_get))) (100.0 100.0 20.0))) "AlwaysSpawn" "MultiplyWithRoot" null (`local.PlayeriD`) null))
      (`self.AddPieceToBoardState` _returnvalue (make `IntPoint` (`local.Row`) (`local.Col`))))
    (:`then_1`
      ;[1 1 1] Right
      (bind _output_get_2 (set `local.Col` (select `int` (`local.PlayeriD`) :`0` 7 :`1` 0)))
      (bind _returnvalue_2 (`|SpawnActorFromClass` "/Game/Pieces/BP_RookFigure.BP_RookFigure_C" (`KismetMathLibrary.MakeTransform` (+ (.location (`BlueprintMapLibrary.Map_Find` (`self.TileTransforms`) (make `IntPoint` (`local.Row`) _output_get_2))) (100.0 100.0 20.0))) "AlwaysSpawn" "MultiplyWithRoot" null (`local.PlayeriD`) null))
      (`self.AddPieceToBoardState` _returnvalue_2 (make `IntPoint` (`local.Row`) (`local.Col`))))))

(fn `UserConstructionScript`
  (`self.SpawnGrid` (`self.Spawn Location Center`) (`self.Tile Size`) (`self.Grid Size`)))