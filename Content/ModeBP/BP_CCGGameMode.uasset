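; BP_CCGGameMode is the game mode for a two-player chess match, assigning player IDs on login and spawn points from BP_PlayerStart IDs.
; Once two players join, it spawns a ChessEngine actor at the standard opening position and starts the first turn.
; CycleTurns submits the current controller's move to the engine, mirrors valid moves on BP_Grid, then swaps turns or reports game over; rejected moves restart the same turn.
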(event `self.K2_PostLogin`
  (params (NewPlayer :type "PlayerController Object Reference"))
  (`parent.K2_PostLogin` NewPlayer)
  (bind _returnvalue (`self.GetNumPlayers`))
  (bind _asbp_classic_player_controller (cast `/Game/ModeBP/BP_ClassicPlayerController` NewPlayer))
  (`/Game/ModeBP/BP_ClassicPlayerController.SetPlayerID` _asbp_classic_player_controller (- _returnvalue 1))
  (bind _returnvalue_2 (`self.GetNumPlayers`))
  (if (== _returnvalue_2 2)
    (`self.StartGame`)
    (else
      (`KismetSystemLibrary.PrintText` "[ERROR] Not enough players!" true true (struct :`R` 1.0 :`A` 1.0)))))

(event `StartGame`
  (bind _returnvalue (`|SpawnActorFromClass` "/Script/ChessDev.ChessEngine" (`KismetMathLibrary.MakeTransform` (0.0 0.0 0.0)) "AlwaysSpawn" "MultiplyWithRoot" null null))
  (bind _output_get (set `self.Engine` _returnvalue))
  (`ChessEngine.setBoardPosition` _output_get "rnbqkbnr/pppppppp/8/8/8/8/PPPPPPPP/RNBQKBNR" 255 true true true true 1.0)
  (`/Game/ModeBP/BP_ClassicPlayerController.StartTurn` (`self.PlayerInTurn`)))

(event `CycleTurns`
  (bind _player_controller (`self.PlayerInTurn`))
  (bind _player_controller_2 (`self.PlayerInTurn`))
  (`/Game/ModeBP/BP_ClassicPlayerController.EndTurn` (`self.PlayerInTurn`))
  (bind _returnvalue (`ChessEngine.makeMove` (`self.Engine`) (`/Game/ModeBP/BP_ClassicPlayerController.fromTile` _player_controller_2) (`/Game/ModeBP/BP_ClassicPlayerController.toTile` _player_controller_2) (`KismetMathLibrary.Conv_IntToByte` (`self.CurrentTurn`)) (`/Game/ModeBP/BP_ClassicPlayerController.Figure Type` _player_controller_2)))
  (if _returnvalue
    (bind _returnvalue_2 (`GameplayStatics.GetActorOfClass` "/Game/ModeBP/BP_Grid.BP_Grid_C"))
    (`/Game/ModeBP/BP_Grid.PerformMove` _returnvalue_2 (`/Game/ModeBP/BP_ClassicPlayerController.fromTile` _player_controller) (`/Game/ModeBP/BP_ClassicPlayerController.toTile` _player_controller) (`/Game/ModeBP/BP_ClassicPlayerController.Figure Type` _player_controller))
    (if (`ChessEngine.isGameFinished` (`self.Engine`))
      (`KismetSystemLibrary.PrintText` "Game Finished" true true (struct :`R` 1.0 :`B` 0.795438 :`A` 1.0))
      (else
        (set `self.CurrentTurn` (select `bool` (== (`self.CurrentTurn`) 0) :`true` 1))
        (`/Game/ModeBP/BP_ClassicPlayerController.StartTurn` (`self.PlayerInTurn`))))
    (else
      (`/Game/ModeBP/BP_ClassicPlayerController.StartTurn` (`self.PlayerInTurn`)))))

(fn `ChoosePlayerStart`
  (params (Player :type "Controller Object Reference"))
  (returns (ReturnValue :type "Actor Object Reference"))
  (`self.InitSpawnPoints`)
  (bind _returnvalue (`self.GetNumPlayers`))
  (return (`BlueprintMapLibrary.Map_Find` (`self.SpawnPoints`) _returnvalue)))

(fn `InitSpawnPoints`
  (if (`BlueprintMapLibrary.Map_IsEmpty` (`self.SpawnPoints`))
    (bind _outactors (`GameplayStatics.GetAllActorsOfClass` "/Game/ModeBP/BP_PlayerStart.BP_PlayerStart_C"))
    (for _array_element _outactors
      (`BlueprintMapLibrary.Map_Add` (`self.SpawnPoints`) (`/Game/ModeBP/BP_PlayerStart.GetPlayerID` _array_element) _array_element))))

(fn `UserConstructionScript`)