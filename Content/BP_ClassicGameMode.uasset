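; Game mode for a two-player turn-based game that starts the first turn once the second player logs in.
; Spawn points come from BP_PlayerStart actors, mapped by player ID on first use and picked by current player count.
; CurrentTurn indexes the player controller receiving turn calls.
; CycleTurns ends that controller's turn but resets CurrentTurn to 0 either way and starts no new turn.
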(event `self.K2_PostLogin`
  (params (NewPlayer :type "PlayerController Object Reference"))
  (bind _returnvalue (`self.GetNumPlayers`))
  (if (== _returnvalue 2)
    (`self.StartGame`)))

(event `StartGame`
  (`/Game/BP_ClassicPlayerController.StartTurn` (`self.PlayerInTurn`)))

(event `CycleTurns`
  (`/Game/BP_ClassicPlayerController.EndTurn` (`self.PlayerInTurn`))
  (set `self.CurrentTurn` (select `bool` (== (`self.CurrentTurn`) 0))))

(fn `ChoosePlayerStart`
  (params (Player :type "Controller Object Reference"))
  (returns (ReturnValue :type "Actor Object Reference"))
  (`self.InitSpawnPoints`)
  (bind _returnvalue (`self.GetNumPlayers`))
  (return (`BlueprintMapLibrary.Map_Find` (`self.SpawnPoints`) _returnvalue)))

(fn `InitSpawnPoints`
  (if (`BlueprintMapLibrary.Map_IsEmpty` (`self.SpawnPoints`))
    (bind _outactors (`GameplayStatics.GetAllActorsOfClass` "/Game/BP_PlayerStart.BP_PlayerStart_C"))
    (for _array_element _outactors
      (`BlueprintMapLibrary.Map_Add` (`self.SpawnPoints`) (`/Game/BP_PlayerStart.GetPlayerID` _array_element) _array_element))))

(fn `UserConstructionScript`)